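; Base board-game placement tile that holds one game feature and defines the feature type that counts as a win on it.
; The tile outline material comes from a PlacementConfig data table lookup by win type, at construction and BeginPlay.
; Interacting swaps features between neighboring placements through message calls.
; An added feature snaps to the tile and, on a type match, triggers the event manager's win check.
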(event `self.ReceiveBeginPlay`
  (`PrimitiveComponent.SetMaterial` (`self.TileOutline`) 0 (`self.PlacementMaterialByType` (`.WinFeatureType_8_31E2F38A4FB61A51F79788A24DECB903` (break `/Game/LestaAcademy/Blueprint/Struct/F_PlacementInfo` (`self.PlacementInfo`))))))

(event `self.Add Object In Placement`
  (params (GameObject :type "Actor Object Reference"))
  (bind _asbp_game_feature (cast `/Game/LestaAcademy/Blueprint/Gameplay/BoardGameObjects/BoardGameObjects/BP_GameFeature` GameObject))
  (bind _output_get (set `self.OwningGameFeature` _asbp_game_feature))
  (message `/Game/LestaAcademy/Blueprint/Interface/BPI_BoardObject.Set Object Placement` _output_get self)
  (`self.K2_SetActorLocation` (`self.OwningGameFeature`) (`self.K2_GetActorLocation`) false false)
  (if (`|EnumEquality` (`.FeatureType_2_ACAE04394F259FF73E9E0C85AD797F3C` (break `/Game/LestaAcademy/Blueprint/Struct/F_GameFeatureInfo` (`/Game/LestaAcademy/Blueprint/Gameplay/BoardGameObjects/BoardGameObjects/BP_GameFeature.GetFeatureInfo` (`self.OwningGameFeature`)))) (`.WinFeatureType_8_31E2F38A4FB61A51F79788A24DECB903` (break `/Game/LestaAcademy/Blueprint/Struct/F_PlacementInfo` (`self.PlacementInfo`))))
    (`/Game/LestaAcademy/Blueprint/Core/BP_EventManager.OnCheckPlacementOnWin` (`/Game/LestaAcademy/Blueprint/FunctionLibraries/BPFL_Events.Get Event Manager`))))

(event `self.ReturnActorToDefaultPlacement`
  (`self.K2_SetActorLocation` (`self.OwningGameFeature`) (`self.K2_GetActorLocation`) false false))

(fn `CancelInteract`
  (returns (bIsReturnToDefaultState :type Boolean))
  (return false))

(fn `Get Object From Placement`
  (returns (BoardGameObject :type "Actor Object Reference"))
  (return (`self.OwningGameFeature`)))

(fn `GetNeighboringPlaces`
  (returns (NeighboringPlaces :type "Array of Actor Object Reference"))
  (return (`self.NeighboringPlaces`)))

(fn `GetPlacementInfo`
  (returns (PlacementInfo :type "/Game/LestaAcademy/Blueprint/Struct/F_PlacementInfo Structure"))
  (return (`self.PlacementInfo`)))

(fn `Interacted`
  (params (InteractedActor :type "Actor Object Reference"))
  (returns (bIsInteracted :type Boolean))
  (bind _placement (message `/Game/LestaAcademy/Blueprint/Interface/BPI_BoardObject.Get Object Placement` InteractedActor))
  (bind _neighboringplaces (message `/Game/LestaAcademy/Blueprint/Interface/BPI_Placement.GetNeighboringPlaces` _placement))
  (if (`KismetArrayLibrary.Array_Contains` _neighboringplaces self)
    (bind _removedobject (message `/Game/LestaAcademy/Blueprint/Interface/BPI_Placement.Remove Object from Placement` _placement))
    (bind _removedobject_2 (`self.Remove Object from Placement`))
    (`self.Add Object In Placement` _removedobject)
    (message `/Game/LestaAcademy/Blueprint/Interface/BPI_Placement.Add Object In Placement` _placement _removedobject_2)
    (return true)
    (else
      (return false))))

(fn `PlacementMaterialByType`
  (params (Type :type "/Game/LestaAcademy/Blueprint/Enum/E_GameFeatureType Enum" :default "NewEnumerator0"))
  (returns (Material :type "MaterialInstance Object Reference"))
  (locals (L_FeatureType :type "/Game/LestaAcademy/Blueprint/Enum/E_GameFeatureType Enum" :default "NewEnumerator0"))
  (set `local.L_FeatureType` Type)
  (bind _outrownames (`DataTableFunctionLibrary.GetDataTableRowNames` (`self.PlacementConfig`)))
  (for _array_element _outrownames
    (bind _returnvalue (`|GetDataTableRow` (`self.PlacementConfig`) _array_element)
      (:`then`
        (bind (_winfeaturetype _material) (break `/Game/LestaAcademy/Blueprint/Struct/F_PlacementConfig` _returnvalue))
        (if (`|EnumEquality` (`local.L_FeatureType`) _winfeaturetype)
          (return _material))))))

(fn `Remove Object from Placement`
  (returns (RemovedObject :type "Actor Object Reference"))
  (locals (LObjectInPlacement :type "Actor Object Reference"))
  (set `local.LObjectInPlacement` (`self.OwningGameFeature`))
  (set `self.OwningGameFeature` null)
  (return (`local.LObjectInPlacement`)))

(fn `StartInteract`
  (returns (bIsSuccess :type Boolean))
  (return false))

(fn `UserConstructionScript`
  (`PrimitiveComponent.SetMaterial` (`self.TileOutline`) 0 (`self.PlacementMaterialByType` (`.WinFeatureType_8_31E2F38A4FB61A51F79788A24DECB903` (break `/Game/LestaAcademy/Blueprint/Struct/F_PlacementInfo` (`self.PlacementInfo`))))))