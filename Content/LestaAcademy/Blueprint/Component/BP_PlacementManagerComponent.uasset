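; Manager component for a placement puzzle that populates the board at start and decides when it is won.
; On BeginPlay it gathers all BP_Placement_Base actors, spawning blocks on blocked ones and game features on non-empty ones.
; Feature types are drawn randomly from a count-limited pool and configured through a data table.
; An event manager event triggers the win check, which fires OnWin when correctly placed counts per type match the pool.
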(event `self.ReceiveBeginPlay`
  (`|ExecutionSequence`
    (:`then_0`
      (`self.InitEvents`)
      (bind _outactors (`GameplayStatics.GetAllActorsOfClass` "/Game/LestaAcademy/Blueprint/Gameplay/BoardGameObjects/Placement/BP_Placement_Base.BP_Placement_Base_C"))
      (set `self.AllPlacement` _outactors))
    (:`then_1`
      (`self.FillPlacementGameFeature`))))

(event `OnCheckPlacementOnWin_Event`
  (if (`self.OnCheckPlacementOnWin`)
    (`/Game/LestaAcademy/Blueprint/Core/BP_EventManager.OnWin` (`/Game/LestaAcademy/Blueprint/FunctionLibraries/BPFL_Events.Get Event Manager`))))

(fn `FeatureConfigByType`
  (params (Type :type "/Game/LestaAcademy/Blueprint/Enum/E_GameFeatureType Enum" :default "NewEnumerator0"))
  (returns (FeatureInfo :type "/Game/LestaAcademy/Blueprint/Struct/F_GameFeatureInfo Structure"))
  (locals (L_FeatureType :type "/Game/LestaAcademy/Blueprint/Enum/E_GameFeatureType Enum" :default "NewEnumerator0"))
  (set `local.L_FeatureType` Type)
  (bind _outrownames (`DataTableFunctionLibrary.GetDataTableRowNames` (`self.FeaturesConfig`)))
  (for _array_element _outrownames
    (bind _returnvalue (`|GetDataTableRow` (`self.FeaturesConfig`) _array_element)
      (:`then`
        (if (`|EnumEquality` (`local.L_FeatureType`) (`.FeatureType_2_ACAE04394F259FF73E9E0C85AD797F3C` (break `/Game/LestaAcademy/Blueprint/Struct/F_GameFeatureInfo` _returnvalue)))
          (return _returnvalue))))))

(fn `FillPlacementGameFeature`
  (locals (L_Placement :type "/Game/LestaAcademy/Blueprint/Gameplay/BoardGameObjects/Placement/BP_Placement_Base Object Reference") (L_GameFeaturePool :type "Map of /Game/LestaAcademy/Blueprint/Enum/E_GameFeatureType Enum to Object Object Reference"))
  (set `local.L_GameFeaturePool` (`self.GameFeaturePool`))
  (for _array_element (`self.AllPlacement`)
    (set `local.L_Placement` _array_element)
    (bind _placementinfo (message `/Game/LestaAcademy/Blueprint/Interface/BPI_Placement.GetPlacementInfo` _array_element))
    (bind (_bisblocked _bisempty) (break `/Game/LestaAcademy/Blueprint/Struct/F_PlacementInfo` _placementinfo))
    (if _bisblocked
      (bind _returnvalue (`|SpawnActorFromClass` "/Game/LestaAcademy/Blueprint/Gameplay/BoardGameObjects/BoardGameObjects/BP_Block.BP_Block_C" (`KismetMathLibrary.MakeTransform` (`Actor.K2_GetActorLocation` (`local.L_Placement`)) (struct)) "Undefined" "OverrideRootScale" null null))
      (message `/Game/LestaAcademy/Blueprint/Interface/BPI_Placement.Add Object In Placement` (`local.L_Placement`) _returnvalue)
      (elif (not _bisempty)
        (bind _returnvalue_2 (`|SpawnActorFromClass` "/Game/LestaAcademy/Blueprint/Gameplay/BoardGameObjects/BoardGameObjects/BP_GameFeature.BP_GameFeature_C" (`KismetMathLibrary.MakeTransform` (`Actor.K2_GetActorLocation` (`local.L_Placement`))) "Undefined" "OverrideRootScale" null (`local.L_Placement`) (`self.FeatureConfigByType` (`self.Get Random Feature Type` (`local.L_GameFeaturePool`))) null))
        (message `/Game/LestaAcademy/Blueprint/Interface/BPI_Placement.Add Object In Placement` (`local.L_Placement`) _returnvalue_2)))))

(fn `Get Random Feature Type`
  (params (GameFeaturePool :type "Map of /Game/LestaAcademy/Blueprint/Enum/E_GameFeatureType Enum to Integer (by ref)"))
  (returns (RandomFeatureType :type "/Game/LestaAcademy/Blueprint/Enum/E_GameFeatureType Enum"))
  (locals (L_RandomFeatureType :type "/Game/LestaAcademy/Blueprint/Enum/E_GameFeatureType Enum" :default "NewEnumerator0") (L_GameFeaturePool :type "Map of /Game/LestaAcademy/Blueprint/Enum/E_GameFeatureType Enum to Integer"))
  (bind _returnvalue (- (`BlueprintMapLibrary.Map_Find` GameFeaturePool (`local.L_RandomFeatureType`)) 1))
  (bind _keys (`BlueprintMapLibrary.Map_Keys` GameFeaturePool))
  (set `local.L_RandomFeatureType` (`KismetArrayLibrary.Array_Random` _keys))
  (if (<= _returnvalue 0)
    (`BlueprintMapLibrary.Map_Remove` GameFeaturePool (`local.L_RandomFeatureType`))
    (return (`local.L_RandomFeatureType`))
    (else
      (`BlueprintMapLibrary.Map_Add` GameFeaturePool (`local.L_RandomFeatureType`) _returnvalue)
      (return (`local.L_RandomFeatureType`)))))

(fn `InitEvents`
  (add `/Game/LestaAcademy/Blueprint/Core/BP_EventManager.OnCheckPlacementOnWin` (`/Game/LestaAcademy/Blueprint/FunctionLibraries/BPFL_Events.Get Event Manager`) (`|CreateDelegate` :!event `OnCheckPlacementOnWin_Event`)))

(fn `OnCheckPlacementOnWin`
  (returns (IsWin :type Boolean))
  (locals (L_CheckPool :type "Map of /Game/LestaAcademy/Blueprint/Enum/E_GameFeatureType Enum to Integer"))
  (for _array_element (`self.AllPlacement`)
    (bind _placementinfo (message `/Game/LestaAcademy/Blueprint/Interface/BPI_Placement.GetPlacementInfo` _array_element))
    (bind _boardgameobject (message `/Game/LestaAcademy/Blueprint/Interface/BPI_Placement.Get Object From Placement` _array_element))
    (bind _asbp_game_feature (cast `/Game/LestaAcademy/Blueprint/Gameplay/BoardGameObjects/BoardGameObjects/BP_GameFeature` _boardgameobject))
    (bind ((`FeatureType_2_ACAE04394F259FF73E9E0C85AD797F3C` _featuretype)) (break `/Game/LestaAcademy/Blueprint/Struct/F_GameFeatureInfo` (`/Game/LestaAcademy/Blueprint/Gameplay/BoardGameObjects/BoardGameObjects/BP_GameFeature.GetFeatureInfo` _asbp_game_feature)))
    (bind ((`WinFeatureType_8_31E2F38A4FB61A51F79788A24DECB903` _winfeaturetype)) (break `/Game/LestaAcademy/Blueprint/Struct/F_PlacementInfo` _placementinfo))
    (if (== _featuretype _winfeaturetype)
      (`BlueprintMapLibrary.Map_Add` (`local.L_CheckPool`) _featuretype (+ (`BlueprintMapLibrary.Map_Find` (`local.L_CheckPool`) _winfeaturetype) 1))))
  (bind _keys (`BlueprintMapLibrary.Map_Keys` (`self.GameFeaturePool`)))
  (for _array_element_2 _keys
    (if (!= (`BlueprintMapLibrary.Map_Find` (`self.GameFeaturePool`) _array_element_2) (`BlueprintMapLibrary.Map_Find` (`local.L_CheckPool`) _array_element_2))
      (return false)))
  (return true))