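; Actor component that lets its owner interact with world actors under the mouse and hand them to placement targets.
; It binds to event manager start, end, cancel and mouse-location events, line-tracing from the owner to the cached mouse location.
; Start messages and stores the hit WorldDynamic actor; end passes it to a placement found on a separate object channel.
; Failed placement fires cancel; references are cleared when interaction finishes or fails.
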(event `self.ReceiveBeginPlay`
  (`|ExecutionSequence`
    (:`then_0`
      (`self.InitEvents`))))

(event `OnActorInteractStart_Event`
  (bind _output_get (set `self.Intreract Actor` (`self.InteractedActorDetected` (`self.Intreract Actor`))))
  (bind _bissuccess (message `/Game/LestaAcademy/Blueprint/Interface/BPI_Interact.StartInteract` _output_get))
  (if (not _bissuccess)
    (`self.CleanRef`)))

(event `OnActorInteractEnd_Event`
  (`self.Intreract Actor`
    (:`then`
      (bind _bisinteracted (message `/Game/LestaAcademy/Blueprint/Interface/BPI_Interact.Interacted` (`self.PlacementDetected`) (`self.Intreract Actor`)))
      (if (not _bisinteracted)
        (`self.OnActorInteractCancel_Event` (`self.Intreract Actor`))
        (`self.CleanRef`)
        (else
          (`self.CleanRef`))))
    (:`else`
      (`self.CleanRef`))))

(event `OnActorInteractCancel_Event`
  (params (InteractActor :type "Actor Object Reference") (Area :type "Actor Object Reference"))
  (message `/Game/LestaAcademy/Blueprint/Interface/BPI_Interact.CancelInteract` (`self.Intreract Actor`))
  (`self.CleanRef`))

(event `OnMouseLocationUpdate_Event`
  (params (NewMouseLocation :type "Vector Structure"))
  (set `self.Mouse Location` NewMouseLocation))

(event `CleanRef`
  (set `self.Intreract Actor` null)
  (set `self.PastPlacement` null))

(fn `InitEvents`
  (`|ExecutionSequence`
    (:`then_0`
      (add `/Game/LestaAcademy/Blueprint/Core/BP_EventManager.OnInteractStart` (`/Game/LestaAcademy/Blueprint/FunctionLibraries/BPFL_Events.Get Event Manager`) (`|CreateDelegate` :!event `OnActorInteractStart_Event`)))
    (:`then_1`
      (add `/Game/LestaAcademy/Blueprint/Core/BP_EventManager.OnInteractEnd` (`/Game/LestaAcademy/Blueprint/FunctionLibraries/BPFL_Events.Get Event Manager`) (`|CreateDelegate` :!event `OnActorInteractEnd_Event`)))
    (:`then_2`
      (add `/Game/LestaAcademy/Blueprint/Core/BP_EventManager.OnInteractCancel` (`/Game/LestaAcademy/Blueprint/FunctionLibraries/BPFL_Events.Get Event Manager`) (`|CreateDelegate` :!event `OnActorInteractCancel_Event`)))
    (:`then_3`
      (add `/Game/LestaAcademy/Blueprint/Core/BP_EventManager.OnMouseLocationUpdate` (`/Game/LestaAcademy/Blueprint/FunctionLibraries/BPFL_Events.Get Event Manager`) (`|CreateDelegate` :!event `OnMouseLocationUpdate_Event`)))))

(fn `InteractedActorDetected`
  (params (IgnoredActor :type "Actor Object Reference"))
  (returns (HitActor :type "Actor Object Reference"))
  (locals (WorldLocation :type "Vector Structure") (WorldDirection :type "Vector Structure"))
  (bind _outhit (`KismetSystemLibrary.LineTraceSingleForObjects` (`Actor.K2_GetActorLocation` (`self.GetOwner`)) (`self.Mouse Location`) (`|MakeArray` "ObjectTypeQuery2" :!type "EObjectTypeQuery Enum") false (`|MakeArray` IgnoredActor) "None" true (struct :`R` 1.0 :`A` 1.0) (struct :`G` 1.0 :`A` 1.0) 10.0))
  (return (`.HitActor` (`GameplayStatics.BreakHitResult` _outhit))))

(fn `PlacementDetected`
  (returns (HitActor :type "Actor Object Reference"))
  (locals (WorldLocation :type "Vector Structure") (WorldDirection :type "Vector Structure"))
  (bind _outhit (`KismetSystemLibrary.LineTraceSingleForObjects` :`Start` (`Actor.K2_GetActorLocation` (`self.GetOwner`)) :`End` (`self.Mouse Location`) :`ObjectTypes` (`|MakeArray` "ObjectTypeQuery7" :!type "EObjectTypeQuery Enum") :`DrawTime` 10.0))
  (return (`.HitActor` (`GameplayStatics.BreakHitResult` _outhit))))